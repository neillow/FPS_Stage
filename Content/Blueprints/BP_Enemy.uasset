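; BP_Enemy is an enemy with health, hit feedback and a ragdoll death.
; TakeDamage subtracts a fixed amount of Health and switches to ragdoll at zero or below by enabling mesh physics and disabling capsule collision.
; Each hit also turns the mesh materials' "Hit" vector parameter red, then restores it to white after a short retriggerable delay.
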(event Custom|PlaceRagdoll
  (bind _mesh (Variables|Character|GetMesh))
  (Physics|SetSimulatePhysics _mesh true)
  (Collision|SetCollisionProfileName _mesh "Ragdoll" true :!class /Script/Engine.PrimitiveComponent)
  (Collision|SetCollisionEnabled (Variables|Collision|GetCapsuleComponent) "NoCollision"))

(event Custom|TakeDamage
  (Utilities|FlowControl|Sequence
    (:then_0
      (Variables|Default|SetHealth (- (Variables|Default|GetHealth) 10))
      (if (<= (Variables|Default|GetHealth) 0)
        (CallFunction|PlaceRagdoll)))
    (:then_1
      (Rendering|Material|SetVectorParameterValueonMaterials (Variables|Character|GetMesh) "Hit" "1.000000,0.000000,0.000000")
      (Utilities|FlowControl|RetriggerableDelay 0.08)
      (Rendering|Material|SetVectorParameterValueonMaterials (Variables|Character|GetMesh) "Hit" "1.000000,1.000000,1.000000"))))

(event EventBeginPlay)

(event Collision|EventActorBeginOverlap
  (params (OtherActor :type Actor%20Object%20Reference)))

(fn ConstructionScript)